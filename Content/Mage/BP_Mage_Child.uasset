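; Mage child Blueprint that implements quick and charged spell attacks, two of each.
; Each attack function calls an event that sets a montage and spawn class, then runs the shared CastSpell.
; CastSpell plays the montage, spawns the class at Arrow1 after a delay and briefly shows a hit particle.
; All attacks use BP_Spell except Quick Spell 1, whose class is None.
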(event `CastSpell`
  ;[1 1 1] Cast Spell
  (`self.PlayAnimMontage` (`self.Anim Montage`))
  (`KismetSystemLibrary.Delay` 0.75)
  (`|SpawnActorFromClass` (`self.Class`) (`SceneComponent.K2_GetComponentToWorld` (`self.Arrow1`)) "Undefined" "OverrideRootScale" null null)
  (bind _returnvalue (`GameplayStatics.SpawnEmitterAtLocation` "/Game/FXVarietyPack/Particles/P_ky_hit1.P_ky_hit1" (.location (`SceneComponent.K2_GetComponentToWorld` (`self.ParticleSystem`))) (struct) (0.2 0.2 0.2)))
  (`KismetSystemLibrary.Delay` 0.2)
  (`ActorComponent.K2_DestroyComponent` _returnvalue))

(event `QuickSpell1`
  ;[1 1 1] Quick Spell 1
  (`|ExecutionSequence`
    (:`then_0`
      (set `self.Class` "/Game/Mage/Spells/BP_Spell.BP_Spell_C"))
    (:`then_1`
      (set `self.Anim Montage` "/Game/Mage/Animation/QuickAttack1_AnimMontage.QuickAttack1_AnimMontage"))
    (:`then_2`
      (`self.CastSpell`))))

(event `ChargedSpell1`
  ;[1 1 1] Charged Spell 1
  (`|ExecutionSequence`
    (:`then_0`
      (set `self.Class` "/Game/Mage/Spells/BP_Spell.BP_Spell_C"))
    (:`then_1`
      (set `self.Anim Montage` "/Game/Mage/Animation/StrongAttack1_AnimMontage.StrongAttack1_AnimMontage"))
    (:`then_2`
      (`self.CastSpell`))))

(event `QuickSpell2`
  ;[1 1 1] Quick Spell 2
  (`|ExecutionSequence`
    (:`then_0`
      (set `self.Class` "/Game/Mage/Spells/BP_Spell.BP_Spell_C"))
    (:`then_1`
      (set `self.Anim Montage` "/Game/Mage/Animation/QuickAttack2_AnimMontage.QuickAttack2_AnimMontage"))
    (:`then_2`
      (`self.CastSpell`))))

(event `ChargedSpell2`
  ;[1 1 1] Charged Spell 2
  (`|ExecutionSequence`
    (:`then_0`
      (set `self.Class` "/Game/Mage/Spells/BP_Spell.BP_Spell_C"))
    (:`then_1`
      (set `self.Anim Montage` "/Game/Mage/Animation/StrongAttack2_AnimMontage.StrongAttack2_AnimMontage"))
    (:`then_2`
      (`self.CastSpell`))))

(fn `ChargedAttack1`
  (`self.ChargedSpell1`))

(fn `ChargedAttack2`
  (`self.ChargedSpell2`))

(fn `QuickAttack1`
  (`self.QuickSpell1`))

(fn `QuickAttack2`
  (`self.QuickSpell2`))

(fn `UserConstructionScript`
  (`parent.UserConstructionScript`))