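; Mage character Blueprint that casts four spells through quick and charged attack functions, two of each.
; Each attack function calls a spell event that sets the spell class, montage and delay, then calls a shared CastSpell event with an arrow component.
; CastSpell plays the montage, waits the delay, then spawns the spell actor at that arrow's transform; only the second charged spell uses a different arrow.
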(event `CastSpell`
  (params (Arrow :type "SceneComponent Object Reference"))
  ;[1 1 1] Cast Spell
  (`self.PlayAnimMontage` (`self.Anim Montage`))
  (`KismetSystemLibrary.Delay` (`self.Duration`))
  (`|SpawnActorFromClass` (`self.Spell`) (`SceneComponent.K2_GetComponentToWorld` Arrow) "Undefined" "OverrideRootScale" null null))

(event `QuickSpell1`
  ;[1 1 1] Quick Spell 1
  (`|ExecutionSequence`
    (:`then_0`
      (set `self.Spell` "/Game/Mage/Spells/BP_Spell.BP_Spell_C"))
    (:`then_1`
      (set `self.Anim Montage` "/Game/Mage/Animation/QuickSpell1_AnimMontage.QuickSpell1_AnimMontage"))
    (:`then_2`
      (set `self.Duration` 0.5))
    (:`then_3`
      (`self.CastSpell` (`self.Arrow1`)))))

(event `ChargedSpell1`
  ;[1 1 1] Charged Spell 1
  (`|ExecutionSequence`
    (:`then_0`
      (set `self.Spell` "/Game/Mage/Spells/BP_Spell2.BP_Spell2_C"))
    (:`then_1`
      (set `self.Anim Montage` "/Game/Mage/Animation/StrongSpell1_AnimMontage.StrongSpell1_AnimMontage"))
    (:`then_2`
      (set `self.Duration` 1.4))
    (:`then_3`
      (`self.CastSpell` (`self.Arrow1`)))))

(event `QuickSpell2`
  ;[1 1 1] Quick Spell 2
  (`|ExecutionSequence`
    (:`then_0`
      (set `self.Spell` "/Game/Mage/Spells/BP_Spell1.BP_Spell1_C"))
    (:`then_1`
      (set `self.Anim Montage` "/Game/Mage/Animation/QuickSpell2_AnimMontage.QuickSpell2_AnimMontage"))
    (:`then_2`
      (set `self.Duration` 0.3))
    (:`then_3`
      (`self.CastSpell` (`self.Arrow1`)))))

(event `ChargedSpell2`
  ;[1 1 1] Charged Spell 2
  (`|ExecutionSequence`
    (:`then_0`
      (set `self.Spell` "/Game/Mage/Spells/BP_Spell3.BP_Spell3_C"))
    (:`then_1`
      (set `self.Anim Montage` "/Game/Mage/Animation/StrongSpell2_AnimMontage.StrongSpell2_AnimMontage"))
    (:`then_2`
      (set `self.Duration` 1.9))
    (:`then_3`
      (`self.CastSpell` (`self.Arrow2`)))))

(fn `ChargedAttack1`
  (`self.ChargedSpell1`))

(fn `ChargedAttack2`
  (`self.ChargedSpell2`))

(fn `QuickAttack1`
  (`self.QuickSpell1`))

(fn `QuickAttack2`
  (`self.QuickSpell2`))

(fn `UserConstructionScript`
  (`parent.UserConstructionScript`))