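; Capoeirista character Blueprint that performs four attacks: quick and charged variants of a punch and a kick.
; The quick and charged attack functions each call an event that pairs an animation montage with an elemental particle effect.
; Punches and kicks use separate particle components, swapping templates per move and deactivating them after timed delays.
; Quick attacks delay before playing their montage, while strong attacks play it immediately.
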(event `QuickPunch`
  (bind _particlesystem (`self.ParticleSystem`))
  (`ParticleSystemComponent.SetTemplate` _particlesystem "/Game/InfinityBladeEffects/Effects/FX_Mobile/Fire/combat/P_AOE_Fire_CircleAttack.P_AOE_Fire_CircleAttack")
  (`KismetSystemLibrary.Delay` 0.7)
  (`self.PlayAnimMontage` "/Game/Capoeirista/Animation/QuickPunch_AnimMontage.QuickPunch_AnimMontage" 1.0 "None")
  (`ActorComponent.Deactivate` _particlesystem))

(event `QuickKick`
  (bind _particlesystem1 (`self.ParticleSystem1`))
  (`ParticleSystemComponent.SetTemplate` _particlesystem1 "/Game/InfinityBladeEffects/Effects/FX_Mobile/ICE/combat/P_AOE_Ice_CircleAttack.P_AOE_Ice_CircleAttack")
  (`KismetSystemLibrary.Delay` 1.3)
  (`self.PlayAnimMontage` "/Game/Capoeirista/Animation/QuickKick_AnimMontage.QuickKick_AnimMontage")
  (`ActorComponent.Deactivate` _particlesystem1))

(event `StrongPunch`
  (bind _particlesystem (`self.ParticleSystem`))
  (`ParticleSystemComponent.SetTemplate` _particlesystem "/Game/FXVarietyPack/Particles/P_ky_thunderBall.P_ky_thunderBall")
  (`self.PlayAnimMontage` "/Game/Capoeirista/Animation/StrongPunch_AnimMontage.StrongPunch_AnimMontage")
  (`KismetSystemLibrary.Delay` 1.4)
  (`ActorComponent.Deactivate` _particlesystem))

(event `StrongKick`
  (bind _particlesystem1 (`self.ParticleSystem1`))
  (`ParticleSystemComponent.SetTemplate` _particlesystem1 "/Game/InfinityBladeEffects/Effects/FX_Forging/P_ForgeDip_Firey.P_ForgeDip_Firey")
  (`self.PlayAnimMontage` "/Game/Capoeirista/Animation/Martelo_Do_Chau_Montage.Martelo_Do_Chau_Montage")
  (`KismetSystemLibrary.Delay` 1.5)
  (`ActorComponent.Deactivate` _particlesystem1))

(fn `ChargedAttack1`
  (`self.StrongPunch`))

(fn `ChargedAttack2`
  (`self.StrongKick`))

(fn `QuickAttack1`
  (`self.QuickPunch`))

(fn `QuickAttack2`
  (`self.QuickKick`))

(fn `UserConstructionScript`)