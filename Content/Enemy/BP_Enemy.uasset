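; BP_Enemy is an enemy with four melee attack events: quick and strong punches and kicks, each stronger than the last.
; Each shows a particle effect, plays a hit sound and montage, and sets damage plus DamageBoost.
; Quick attacks delay before the montage as a wind-up, while strong attacks delay after starting it.
; Attack then sphere-traces a short distance forward and calls ReduceLife on any BP_ParentCharacter hit.
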(event `QuickPunch`
  (bind _particlesystem (`self.ParticleSystem`))
  ;[1 1 1] Play attacks
  (`ParticleSystemComponent.SetTemplate` _particlesystem "/Game/InfinityBladeEffects/Effects/FX_Mobile/Fire/combat/P_AOE_Fire_CircleAttack.P_AOE_Fire_CircleAttack")
  (`KismetSystemLibrary.Delay` 0.7)
  (`GameplayStatics.SpawnSoundAttached` "/Game/Sounds/hit.hit" (`self.Mesh`) "None" (0.0 0.0 0.0) (struct) "KeepRelativeOffset" false 1.0 1.0 0.0 null null)
  (`self.PlayAnimMontage` "/Game/Capoeirista/Animation/QuickPunch_AnimMontage.QuickPunch_AnimMontage" 1.0 "None")
  (`ActorComponent.Deactivate` _particlesystem)
  (set `self.Damage` (+ 5 (`self.DamageBoost`)))
  (`self.Attack`))

(event `QuickKick`
  (bind _particlesystem1 (`self.ParticleSystem1`))
  ;[1 1 1] Play attacks
  (`ParticleSystemComponent.SetTemplate` _particlesystem1 "/Game/InfinityBladeEffects/Effects/FX_Mobile/ICE/combat/P_AOE_Ice_CircleAttack.P_AOE_Ice_CircleAttack")
  (`KismetSystemLibrary.Delay` 1.3)
  (`GameplayStatics.SpawnSoundAttached` "/Game/Sounds/hit.hit" (`self.Mesh`) "None" (0.0 0.0 0.0) (struct) "KeepRelativeOffset" false 1.0 1.0 0.0 null null)
  (`self.PlayAnimMontage` "/Game/Capoeirista/Animation/QuickKick_AnimMontage.QuickKick_AnimMontage")
  (`ActorComponent.Deactivate` _particlesystem1)
  (set `self.Damage` (+ 10 (`self.DamageBoost`)))
  (`self.Attack`))

(event `StrongPunch`
  (bind _particlesystem (`self.ParticleSystem`))
  ;[1 1 1] Play attacks
  (`ParticleSystemComponent.SetTemplate` _particlesystem "/Game/FXVarietyPack/Particles/P_ky_thunderBall.P_ky_thunderBall")
  (`GameplayStatics.SpawnSoundAttached` "/Game/Sounds/hit.hit" (`self.Mesh`) "None" (0.0 0.0 0.0) (struct) "KeepRelativeOffset" false 1.0 1.0 0.0 null null)
  (`self.PlayAnimMontage` "/Game/Capoeirista/Animation/StrongPunch_AnimMontage.StrongPunch_AnimMontage")
  (`KismetSystemLibrary.Delay` 1.4)
  (`ActorComponent.Deactivate` _particlesystem)
  (set `self.Damage` (+ 15 (`self.DamageBoost`)))
  (`self.Attack`))

(event `StrongKick`
  (bind _particlesystem1 (`self.ParticleSystem1`))
  ;[1 1 1] Play attacks
  (`ParticleSystemComponent.SetTemplate` _particlesystem1 "/Game/InfinityBladeEffects/Effects/FX_Forging/P_ForgeDip_Firey.P_ForgeDip_Firey")
  (`GameplayStatics.SpawnSoundAttached` "/Game/Sounds/hit.hit" (`self.Mesh`) "None" (0.0 0.0 0.0) (struct) "KeepRelativeOffset" false 1.0 1.0 0.0 null null)
  (`self.PlayAnimMontage` "/Game/Capoeirista/Animation/StrongKick_AnimMontage.StrongKick_AnimMontage")
  (`KismetSystemLibrary.Delay` 1.5)
  (`ActorComponent.Deactivate` _particlesystem1)
  (set `self.Damage` (+ 20 (`self.DamageBoost`)))
  (`self.Attack`))

(event `Attack`
  (bind _returnvalue (`self.K2_GetActorLocation`))
  ;[1 1 1] Trace attack
  (bind _outhit (`KismetSystemLibrary.SphereTraceSingle` _returnvalue (+ _returnvalue (* (`self.GetActorForwardVector`) 100.0)) 50.0 "TraceTypeQuery1" true))
  (bind _asbp_parent_character (cast `/Game/SideScrollerBP/Blueprints/BP_ParentCharacter` (`.HitActor` (`GameplayStatics.BreakHitResult` _outhit))))
  (`self.ReduceLife` _asbp_parent_character (`self.Damage`)))

(fn `UserConstructionScript`)